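; BP_Sandik is a breakable loot container that is destroyed when it takes damage and may drop an item.
; Its damage event rolls a random integer over four equally likely outcomes: two spawn either a kunai or a can item, and two drop nothing.
; Drops spawn slightly above the container's location, and every outcome destroys the actor, with no check on the damage amount.
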(event EventBeginPlay)

(event Collision|EventActorBeginOverlap
  (params (OtherActor :type Actor%20Object%20Reference)))

(event EventTick
  (params (DeltaSeconds :type Float%20%28single-precision%29)))

(event EventTakeDamage
  (params (DamageCauser :type Actor%20Object%20Reference) (SelectedDamage :type Float%20%28double-precision%29))
  (bind _returnvalue (Transformation|GetActorLocation))
  (bind _returnvalue_2 (+ _returnvalue "0.000000,0.000000,100.000000"))
  (switch int (Math|Random|RandomIntegerinRange 0 3)
    (:0
      (Game|SpawnActorfromClass "/Game/blueprint/BP_Item_Kunai.BP_Item_Kunai_C" (Math|Conversions|ToTransform(Vector) _returnvalue_2) "Undefined" "MultiplyWithRoot" 0 0)
      (Actor|DestroyActor))
    (:1
      (Game|SpawnActorfromClass "/Game/blueprint/BP_Item_Can.BP_Item_Can_C" (Math|Conversions|ToTransform(Vector) _returnvalue_2) "Undefined" "MultiplyWithRoot" 0 0)
      (Actor|DestroyActor))
    (:2
      (Actor|DestroyActor))
    (:3
      (Actor|DestroyActor))))

(fn ConstructionScript)