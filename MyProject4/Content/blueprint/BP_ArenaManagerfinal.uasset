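; Arena manager that locks the player between two side barriers on first trigger overlap and runs a series of enemy waves.
; Each wave takes its count from a list and spawns enemies at three random points with X jitter, targeting the player.
; Enemy destruction callbacks count kills to start the next wave after a delay, or open the barriers after the last.
; A reset event clears enemies and progress, re-arms the trigger and briefly suppresses wave advancement.
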(event OnComponentBeginOverlap(Box)
  (params (OverlappedComponent :type Primitive%20Component%20Object%20Reference) (OtherActor :type Actor%20Object%20Reference) (OtherComp :type Primitive%20Component%20Object%20Reference) (OtherBodyIndex :type Integer) (bFromSweep :type Boolean) (SweepResult :type Hit%20Result%20Structure%20%28by%20ref%29))
  (if (Actor|ActorHasTag OtherActor "Player")
    (Utilities|FlowControl|DoOnce false
      (:Completed
        (Collision|SetCollisionEnabled (Variables|Default|Getsağ) "QueryAndPhysics")
        (CallFunction|DalgayiBaslat)
        (for _index (range 1 (Variables|Default|GetDalgaHedefi))
          (bind _returnvalue (Game|SpawnActorfromClass "/Game/charecters/enemy.enemy_C" (Math|Transform|MakeTransform (+ (Utilities|Select :Index (Math|Random|RandomIntegerinRange 0 2) :Option%200 (.location (Transformation|GetWorldTransform (Variables|Default|GetSpawnNoktasi_1))) :Option%201 (.location (Transformation|GetWorldTransform (Variables|Default|GetSpawnNoktasi_3))) :Option%202 (.location (Transformation|GetWorldTransform (Variables|Default|GetSpawnNoktasi_2)))) (Math|Vector|MakeVector (Math|Random|RandomFloatinRange -5e+01 5e+01) 0.0 0.0)) "0, 0, 0" "1.000000,1.000000,1.000000") "AlwaysSpawn" "MultiplyWithRoot" 0 (Game|GetPlayerCharacter 0) 0))
          (Utilities|Array|Add (Variables|Default|GetSahnedekiDusmanlar) _returnvalue)
          (Game|BindEventtoOnDestroyed _returnvalue (delegate Custom|DusmanOldu)))))))

(event Custom|ArenaSifirla
  (for _array_element (Variables|Default|GetSahnedekiDusmanlar)
    (if (Utilities|IsValid _array_element)
      (Actor|DestroyActor _array_element)
      (Collision|SetCollisionEnabled (Variables|Default|Getsağ) "NoCollision")))
  (Utilities|Array|Clear (Variables|Default|GetSahnedekiDusmanlar))
  (Variables|Default|SetToplamDusmanSayisi 0)
  (Variables|Default|SetOlenDusmanSayisi 0)
  (Variables|Default|SetSuankiDalgaIndex 0)
  (Utilities|FlowControl|DoOnce false) ; enters at Reset
)

(event Custom|DusmanOldu
  (params (DestroyedActor :type Actor%20Object%20Reference))
  (Math|Integer|IncrementInt (Variables|Default|GetOlenDusmanSayisi)
    (:%20%20
      (if (== (Variables|Default|GetOlenDusmanSayisi) (Variables|Default|GetDalgaHedefi))
        (Math|Integer|IncrementInt (Variables|Default|GetSuankiDalgaIndex)
          (:%20%20
            (if (< (Variables|Default|GetSuankiDalgaIndex) (Utilities|Array|Length (Variables|Default|GetDalgaListesi)))
              (if (not (Variables|Default|Getkarakter%20ölümğ))
                (Utilities|FlowControl|Delay 1.0)
                (CallFunction|Sinyal))
              (else
                (Collision|SetCollisionEnabled (Variables|Default|Getsağ) "NoCollision")))))))))

(event Custom|DalgayiBaslat
  (Variables|Default|SetDalgaHedefi (Utilities|Array|Get(acopy) (Variables|Default|GetDalgaListesi) (Variables|Default|GetSuankiDalgaIndex)))
  (Variables|Default|SetOlenDusmanSayisi 0))

(event Custom|sinyal
  (CallFunction|DalgayiBaslat)
  (for _index (range 1 (Variables|Default|GetDalgaHedefi))
    (bind _returnvalue (Game|SpawnActorfromClass "/Game/charecters/enemy.enemy_C" (Math|Transform|MakeTransform (+ (Utilities|Select :Index (Math|Random|RandomIntegerinRange 0 2) :Option%200 (.location (Transformation|GetWorldTransform (Variables|Default|GetSpawnNoktasi_1))) :Option%201 (.location (Transformation|GetWorldTransform (Variables|Default|GetSpawnNoktasi_3))) :Option%202 (.location (Transformation|GetWorldTransform (Variables|Default|GetSpawnNoktasi_2)))) (Math|Vector|MakeVector (Math|Random|RandomFloatinRange -5e+01 5e+01) 0.0 0.0)) "0, 0, 0" "1.000000,1.000000,1.000000") "AlwaysSpawn" "MultiplyWithRoot" 0 (Game|GetPlayerCharacter 0) 0))
    (Utilities|Array|Add (Variables|Default|GetSahnedekiDusmanlar) _returnvalue)
    (Game|BindEventtoOnDestroyed _returnvalue (delegate Custom|DusmanOldu))))

(event EventBeginPlay)

(event Collision|EventActorBeginOverlap
  (params (OtherActor :type Actor%20Object%20Reference)))

(event EventIResetMe
  (CallFunction|ArenaSifirla)
  (Variables|Default|Setkarakter%20ölümğ true)
  (Utilities|FlowControl|Delay 1.0)
  (Variables|Default|Setkarakter%20ölümğ false))

(fn ConstructionScript)