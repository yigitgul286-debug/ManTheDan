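; BP_ArenaManager runs a lock-in combat arena that traps the player until every spawned enemy is gone.
; The first player overlap with its Box enables collision on the Sağ and Sol barriers and spawns enemies targeting the player at three random points, jittered along X.
; Each enemy's OnDestroyed feeds a death counter that disables the barriers at the total.
; IResetMe destroys remaining enemies, clears the count and re-arms the DoOnce trigger.
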(event OnComponentBeginOverlap(Box)
  (params (OverlappedComponent :type Primitive%20Component%20Object%20Reference) (OtherActor :type Actor%20Object%20Reference) (OtherComp :type Primitive%20Component%20Object%20Reference) (OtherBodyIndex :type Integer) (bFromSweep :type Boolean) (SweepResult :type Hit%20Result%20Structure%20%28by%20ref%29))
  (if (Actor|ActorHasTag OtherActor "Player")
    (Utilities|FlowControl|DoOnce false
      (:Completed
        (Collision|SetCollisionEnabled (Variables|Default|Getsağ) "QueryAndPhysics")
        (for _index (range 1 (Variables|Default|GetToplamDusmanSayisi))
          (bind _returnvalue (Game|SpawnActorfromClass "/Game/charecters/enemy.enemy_C" (Math|Transform|MakeTransform (+ (Utilities|Select :Index (Math|Random|RandomIntegerinRange 0 2) :Option%200 (.location (Transformation|GetWorldTransform (Variables|Default|GetSpawnNoktasi_1))) :Option%201 (.location (Transformation|GetWorldTransform (Variables|Default|GetSpawnNoktasi_3))) :Option%202 (.location (Transformation|GetWorldTransform (Variables|Default|GetSpawnNoktasi_2)))) (Math|Vector|MakeVector (Math|Random|RandomFloatinRange -5e+01 5e+01) 0.0 0.0)) "0, 0, 0" "1.000000,1.000000,1.000000") "AlwaysSpawn" "MultiplyWithRoot" 0 (Game|GetPlayerCharacter 0) 0))
          (Utilities|Array|Add (Variables|Default|GetSahnedekiDusmanlar) _returnvalue)
          (Game|BindEventtoOnDestroyed _returnvalue (delegate Custom|DusmanOldu)))))))

(event Custom|ArenaSifirla
  (for _array_element (Variables|Default|GetSahnedekiDusmanlar)
    (if (Utilities|IsValid _array_element)
      (Actor|DestroyActor _array_element)))
  (Utilities|Array|Clear (Variables|Default|GetSahnedekiDusmanlar))
  (Variables|Default|SetOlenDusmanSayisi 0)
  (Utilities|FlowControl|DoOnce false) ; enters at Reset
)

(event Custom|DusmanOldu
  (params (DestroyedActor :type Actor%20Object%20Reference))
  (Math|Integer|IncrementInt (Variables|Default|GetOlenDusmanSayisi)
    (:%20%20
      (if (== (Variables|Default|GetToplamDusmanSayisi) (Variables|Default|GetOlenDusmanSayisi))
        (Collision|SetCollisionEnabled (Variables|Default|Getsağ) "NoCollision")))))

(event EventBeginPlay)

(event Collision|EventActorBeginOverlap
  (params (OtherActor :type Actor%20Object%20Reference)))

(event EventIResetMe
  (CallFunction|ArenaSifirla))

(fn ConstructionScript)