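; One-way platform actor that lets characters pass through it and also moves vertically.
; Overlapping the Box trigger switches off the Cube's collision once; leaving it restores collision after a short delay and re-arms the DoOnce.
; On BeginPlay a Timeline lerps the actor from its start location along Z by HareketMesafesi (movement distance).
; The YukariAssagi (up-down) tile map is assigned in both the construction script and BeginPlay.
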(event OnComponentBeginOverlap(Box)
  (params (OverlappedComponent :type Primitive%20Component%20Object%20Reference) (OtherActor :type Actor%20Object%20Reference) (OtherComp :type Primitive%20Component%20Object%20Reference) (OtherBodyIndex :type Integer) (bFromSweep :type Boolean) (SweepResult :type Hit%20Result%20Structure%20%28by%20ref%29))
  (Utilities|FlowControl|DoOnce false
    (:Completed
      (Collision|SetCollisionEnabled (Variables|Default|GetCube) "NoCollision"))))

(event OnComponentEndOverlap(Box)
  (params (OverlappedComponent :type Primitive%20Component%20Object%20Reference) (OtherActor :type Actor%20Object%20Reference) (OtherComp :type Primitive%20Component%20Object%20Reference) (OtherBodyIndex :type Integer))
  (Utilities|FlowControl|Delay 0.2)
  (Collision|SetCollisionEnabled (Variables|Default|GetCube) "QueryAndPhysics")
  (Utilities|FlowControl|DoOnce false) ; enters at Reset
)

(event Collision|EventActorBeginOverlap
  (params (OtherActor :type Actor%20Object%20Reference)))

(event EventTick
  (params (DeltaSeconds :type Float%20%28single-precision%29)))

(event EventBeginPlay
  (Class|PaperTileMapComponent|SetTileMap (Variables|Default|GetYukariAssagi) "/Game/sprites/Hareketli_Objeler/YukariAssagi.YukariAssagi")
  (bind _output_get (Variables|Default|SetBaslangic%20Konumu (Transformation|GetActorLocation)))
  (bind _newtrack_0 (Timeline|Timeline Play)
    (:Update
      (Transformation|SetActorLocation (Math|Vector|Lerp(Vector) _output_get (+ _output_get (Math|Vector|MakeVector 0.0 0.0 (Variables|Default|GetHareket%20Mesafesi))) _newtrack_0) false false))))

(fn ConstructionScript
  (Class|PaperTileMapComponent|SetTileMap (Variables|Default|GetYukariAssagi) "/Game/sprites/Hareketli_Objeler/YukariAssagi.YukariAssagi"))