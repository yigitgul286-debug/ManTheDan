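; A breakable block actor, apparently for a dungeon level, that is destroyed after taking enough hits.
; Each damage event prints a debug "Hello", lowers BlockHP by one regardless of damage amount, and destroys the actor once HP reaches zero or below.
; The construction script sets the tile map on its 7BlokKirilan component.
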(event EventBeginPlay)

(event Collision|EventActorBeginOverlap
  (params (OtherActor :type Actor%20Object%20Reference)))

(event EventTick
  (params (DeltaSeconds :type Float%20%28single-precision%29)))

(event EventTakeDamage
  (params (DamageCauser :type Actor%20Object%20Reference) (SelectedDamage :type Float%20%28double-precision%29))
  (Development|PrintString "Hello")
  (Variables|Default|SetBlockHP (- (Variables|Default|GetBlockHP) 1))
  (if (<= (Variables|Default|GetBlockHP) 0)
    (Actor|DestroyActor)))

(fn ConstructionScript
  (Class|PaperTileMapComponent|SetTileMap (Variables|Default|Get7BlokKirilan) "/Game/sprites/Hareketli_Objeler/7BlokKirilan.7BlokKirilan"))