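; BP_SOLSAGGİDİS is a tile map actor that moves horizontally along world X, its name being Turkish for left-right movement.
; Construction and BeginPlay both assign the tile map on the YukariAssagi component.
; BeginPlay stores the start location, then a Timeline lerps the actor between it and a point HareketMesafesi away on X, without sweeping.
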(event Collision|EventActorBeginOverlap
  (params (OtherActor :type Actor%20Object%20Reference)))

(event EventTick
  (params (DeltaSeconds :type Float%20%28single-precision%29)))

(event EventBeginPlay
  (Class|PaperTileMapComponent|SetTileMap (Variables|Default|GetYukariAssagi) "/Game/sprites/Hareketli_Objeler/YukariAssagi.YukariAssagi")
  (bind _output_get (Variables|Default|SetBaslangic%20Konumu (Transformation|GetActorLocation)))
  (bind _newtrack_0 (Timeline|Timeline Play)
    (:Update
      (Transformation|SetActorLocation (Math|Vector|Lerp(Vector) _output_get (+ _output_get (Math|Vector|MakeVector (Variables|Default|GetHareket%20Mesafesi) 0.0 0.0)) _newtrack_0) false false))))

(fn ConstructionScript
  (Class|PaperTileMapComponent|SetTileMap (Variables|Default|GetYukariAssagi) "/Game/sprites/Hareketli_Objeler/YukariAssagi.YukariAssagi"))