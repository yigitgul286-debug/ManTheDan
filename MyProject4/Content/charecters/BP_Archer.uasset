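; BP_Archer is a 2D flipbook enemy that shoots arrows at the player and is destroyed by any damage.
; A Box overlap with the Player-tagged actor toggles a flag that lets Tick set a looping timer and call the attack sequence.
; The sequence plays the attack flipbook, waits, then SpawnArrow turns the archer by relative X and spawns BP_Arrow aimed from the muzzle at the player, before returning to idle.
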(event OnComponentBeginOverlap(Box)
  (params (OverlappedComponent :type Primitive%20Component%20Object%20Reference) (OtherActor :type Actor%20Object%20Reference) (OtherComp :type Primitive%20Component%20Object%20Reference) (OtherBodyIndex :type Integer) (bFromSweep :type Boolean) (SweepResult :type Hit%20Result%20Structure%20%28by%20ref%29))
  (if (Actor|ActorHasTag OtherActor "Player")
    (Variables|Default|Setıscasıng true)))

(event OnComponentEndOverlap(Box)
  (params (OverlappedComponent :type Primitive%20Component%20Object%20Reference) (OtherActor :type Actor%20Object%20Reference) (OtherComp :type Primitive%20Component%20Object%20Reference) (OtherBodyIndex :type Integer))
  (if (Actor|ActorHasTag OtherActor "Player")
    (Variables|Default|Setıscasıng false)))

(event Custom|SpawnArrow
  (if (< (.x (Transformation|GetActorLocation)) (.x (Transformation|GetActorLocation (Game|GetPlayerCharacter 0))))
    (Transformation|SetActorRotation (Math|Rotator|MakeRotator 0.0 0.0 0.0))
    (else
      (Transformation|SetActorRotation (Math|Rotator|MakeRotator 0.0 0.0 1.8e+02))))
  (Game|SpawnActorfromClass "/Game/blueprint/BP_Arrow.BP_Arrow_C" (Math|Transform|MakeTransform (Transformation|GetWorldLocation (Variables|Default|GetMuzzleLocation)) (Math|Rotator|FindLookatRotation (Transformation|GetWorldLocation (Variables|Default|GetMuzzleLocation)) (Transformation|GetActorLocation (Game|GetPlayerCharacter 0))) "1.000000,1.000000,1.000000") "Undefined" "MultiplyWithRoot" 0 0))

(event Custom|StartAttackSequence
  (Sprite|SetFlipbook (Variables|Default|GetSoldier-Idle1) "/Game/sprites/enemy1/Soldier-Attack04.Soldier-Attack04")
  (Utilities|FlowControl|Delay 1.6)
  (CallFunction|SpawnArrow)
  (Utilities|FlowControl|Delay 1.6)
  (Sprite|SetFlipbook (Variables|Default|GetSoldier-Idle1) "/Game/sprites/enemy1/Soldier-Idle1.Soldier-Idle1"))

(event EventTick
  (params (DeltaSeconds :type Float%20%28single-precision%29))
  (if (Variables|Default|Getıscasıng)
    (bind _returnvalue (Utilities|Time|SetTimerbyEvent 0 2.0 true))
    (Variables|Default|SetFireTimerRef _returnvalue)
    (if (Collision|IsOverlappingActor (Variables|Default|GetBox) (Game|GetPlayerCharacter 0) :!class /Script/Engine.PrimitiveComponent)
      (CallFunction|StartAttackSequence)
      (else
        (Utilities|Time|ClearandInvalidateTimerbyHandle (Variables|Default|GetFireTimerRef))
        (Sprite|SetFlipbook (Variables|Default|GetSoldier-Idle1) "/Game/sprites/enemy1/Soldier-Idle1.Soldier-Idle1")))))

(event EventTakeDamage
  (params (DamageCauser :type Actor%20Object%20Reference) (SelectedDamage :type Float%20%28double-precision%29))
  (Actor|DestroyActor))

(fn ConstructionScript)